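; Player controller Blueprint for VladMenus that owns the menu interface and feeds it key input.
; On BeginPlay, remote instances, and authority instances that are the first player controller off a dedicated server, set game-only input and add a WBP_Manager widget to the viewport.
; Any key press or release is forwarded to that widget, which is removed on EndPlay.
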(event EventEndPlay
  (params (EndPlayReason :type EEndPlayReason%20Enum :default "Destroyed"))
  (bind _userinterface (Variables|Default|GetUserInterface))
  ;[1 1 1] EndPlay
  ;[1 1 1] Destroy the user interface.
  (Utilities|IsValid _userinterface
    (:Is%20Valid
      (Widget|RemovefromParent _userinterface))))

(event EventBeginPlay
  (bind _returnvalue (Game|GetPlayerController 0))
  ;[1 1 1] BeginPlay
  ;[1 1 1] Create the user interface.
  (Networking|SwitchHasAuthority
    (:Authority
      (if (and (not (Networking|IsDedicatedServer)) (== self _returnvalue))
        (Input|SetInputModeGameOnly _returnvalue :!label _label)
        (bind _returnvalue_2 (UserInterface|CreateWidget "/Game/OpenTournament/VladMenus/World/WBP_Manager.WBP_Manager_C" _returnvalue))
        (bind _output_get (Variables|Default|SetUserInterface _returnvalue_2))
        (UserInterface|Viewport|AddtoViewport _output_get 0)))
    (:Remote
      (goto _label))))

(event Input|KeyboardEvents|AnyKey
  (params (Key :type Key%20Structure))
  (bind _userinterface (Variables|Default|GetUserInterface))
  ;[1 1 1] Hook used by the interface.
  (:Pressed
    (Utilities|IsValid _userinterface
      (:Is%20Valid
        (Default|AnyKeyPressed _userinterface Key))))
  (:Released
    (Utilities|IsValid _userinterface
      (:Is%20Valid
        (Default|AnyKeyReleased _userinterface Key)))))

(fn ConstructionScript)