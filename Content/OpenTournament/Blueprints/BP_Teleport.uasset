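; BP_Teleport is a teleporter that moves characters entering its capsule to a target actor and plays sounds at both ends.
; Yaw is either forced to the target's or offset by it, then applied to actor and control rotation.
; Cached velocity is restored with scaling, without being rotated.
; If the target is another BP_Teleport, it ignores the arriving PlayerState until capsule overlap ends, preventing bounce-back.
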(event OnComponentBeginOverlap(Capsule)
  (params (OverlappedComponent :type Primitive%20Component%20Object%20Reference) (OtherActor :type Actor%20Object%20Reference) (OtherComp :type Primitive%20Component%20Object%20Reference) (OtherBodyIndex :type Integer) (bFromSweep :type Boolean) (SweepResult :type Hit%20Result%20Structure%20%28by%20ref%29))
  (if (Utilities|IsValid (Variables|Default|GetTargetActor))
    (bind _ascharacter (Utilities|Casting|CastToCharacter OtherActor))
    (if (== (Utilities|Array|FindItem (Variables|Default|GetIgnoredPlayers) (Variables|/Script/Engine.Pawn|GetPlayerState _ascharacter)) -1)
      (CallFunction|PreTeleport OtherActor (Variables|/Script/Engine.Pawn|GetPlayerState _ascharacter))
      (Transformation|SetActorLocationAndRotation OtherActor (Transformation|GetActorLocation (Variables|Default|GetTargetActor)) (select (Variables|Default|GetbForceRotationYaw) (Math|Rotator|MakeRotator (.Roll (Math|Rotator|BreakRotator (Pawn|GetControlRotation (Pawn|GetController _ascharacter) :!class /Script/Engine.Controller))) (.Pitch (Math|Rotator|BreakRotator (Pawn|GetControlRotation (Pawn|GetController _ascharacter) :!class /Script/Engine.Controller))) (.Yaw (Math|Rotator|BreakRotator (Transformation|GetActorRotation (Variables|Default|GetTargetActor))))) (Math|Rotator|MakeRotator (.Roll (Math|Rotator|BreakRotator (Pawn|GetControlRotation (Pawn|GetController _ascharacter) :!class /Script/Engine.Controller))) (.Pitch (Math|Rotator|BreakRotator (Pawn|GetControlRotation (Pawn|GetController _ascharacter) :!class /Script/Engine.Controller))) (+ (.Yaw (Math|Rotator|BreakRotator (Pawn|GetControlRotation (Pawn|GetController _ascharacter) :!class /Script/Engine.Controller))) (.Yaw (Math|Rotator|BreakRotator (Transformation|GetActorRotation (Variables|Default|GetTargetActor))))))) false true)
      (CallFunction|PostTeleport (Pawn|GetController _ascharacter) (select (Variables|Default|GetbForceRotationYaw) (Math|Rotator|MakeRotator (.Roll (Math|Rotator|BreakRotator (Pawn|GetControlRotation (Pawn|GetController _ascharacter) :!class /Script/Engine.Controller))) (.Pitch (Math|Rotator|BreakRotator (Pawn|GetControlRotation (Pawn|GetController _ascharacter) :!class /Script/Engine.Controller))) (.Yaw (Math|Rotator|BreakRotator (Transformation|GetActorRotation (Variables|Default|GetTargetActor))))) (Math|Rotator|MakeRotator (.Roll (Math|Rotator|BreakRotator (Pawn|GetControlRotation (Pawn|GetController _ascharacter) :!class /Script/Engine.Controller))) (.Pitch (Math|Rotator|BreakRotator (Pawn|GetControlRotation (Pawn|GetController _ascharacter) :!class /Script/Engine.Controller))) (+ (.Yaw (Math|Rotator|BreakRotator (Pawn|GetControlRotation (Pawn|GetController _ascharacter) :!class /Script/Engine.Controller))) (.Yaw (Math|Rotator|BreakRotator (Transformation|GetActorRotation (Variables|Default|GetTargetActor))))))) OtherActor)
      (CallFunction|PlayTeleportEffects))))

(event OnComponentEndOverlap(Capsule)
  (params (OverlappedComponent :type Primitive%20Component%20Object%20Reference) (OtherActor :type Actor%20Object%20Reference) (OtherComp :type Primitive%20Component%20Object%20Reference) (OtherBodyIndex :type Integer))
  (bind _ascharacter (Utilities|Casting|CastToCharacter OtherActor))
  (Utilities|Array|RemoveIndex (Variables|Default|GetIgnoredPlayers) (Utilities|Array|FindItem (Variables|Default|GetIgnoredPlayers) (Variables|/Script/Engine.Pawn|GetPlayerState _ascharacter))))

(event EventBeginPlay)

(event Collision|EventActorBeginOverlap
  (params (OtherActor :type Actor%20Object%20Reference)))

(event EventTick
  (params (DeltaSeconds :type Float%20%28single-precision%29)))

(fn ConstructionScript)

(fn PlayTeleportEffects
  (Audio|PlaySoundatLocation self (Variables|Default|GetTeleportOutSound) (Transformation|GetActorLocation) "0, 0, 0" 1.0 1.0 0.0 0 0 0)
  (Audio|PlaySoundatLocation self (Variables|Default|GetTeleportInSound) (Transformation|GetActorLocation (Variables|Default|GetTargetActor)) "0, 0, 0" 1.0 1.0 0.0 0 0 0))

(fn PreTeleport
  (params (TeleportActor :type Actor%20Object%20Reference) (IgnoreActorState :type Player%20State%20Object%20Reference%20%28by%20ref%29))
  (bind _ascharacter (Utilities|Casting|CastToCharacter TeleportActor)
    (:then
      (Variables|Default|SetCachedVelocity (Variables|/Script/Engine.MovementComponent|GetVelocity (Pawn|GetMovementComponent _ascharacter))))
    (:CastFailed
      _))
  (bind _asbp_teleport (Utilities|Casting|CastToBP_Teleport (Variables|Default|GetTargetActor))
    (:then
      (Utilities|Array|AddUnique (Variables|BP_Teleport_C|GetIgnoredPlayers _asbp_teleport) IgnoreActorState))
    (:CastFailed
      _))
  (return))

(fn PostTeleport
  (params (TeleportedController :type Controller%20Object%20Reference) (ControllerRotation :type Rotator%20%28by%20ref%29) (TeleportedActor :type Actor%20Object%20Reference))
  (Pawn|SetControlRotation TeleportedController ControllerRotation)
  (bind _ascharacter (Utilities|Casting|CastToCharacter TeleportedActor))
  (Variables|/Script/Engine.MovementComponent|SetVelocity (Pawn|GetMovementComponent _ascharacter) (* (Variables|Default|GetCachedVelocity) (Variables|Default|GetVelocityRetainedScale))))