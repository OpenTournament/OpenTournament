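; Grenade projectile that explodes on a fuse timer in OpenTournament.
; A timer set on spawn calls the inherited Explode at the grenade's current location, using its forward vector as the hit normal.
; The first bounce can reset that timer to a bounced fuse duration, with separate flags allowing it to shorten or lengthen the remaining time.
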(event OnProjectileBounce(ProjectileMovementComponent)
  (params (ImpactResult :type Hit%20Result%20Structure%20%28by%20ref%29) (ImpactVelocity :type Vector%20%28by%20ref%29 :default "0, 0, 0"))
  (bind _timerhandle (Variables|Default|GetTimerHandle))
  (bind _bounced_fuse_duration (Variables|Default|GetBounced%20Fuse%20Duration))
  (bind _returnvalue (Utilities|Time|GetTimerRemainingTimebyHandle _timerhandle))
  ;[0 1 1] First bounce updates fuse
  (if (not (Variables|Default|GetBounced))
    (Variables|Default|SetBounced true)
    (if (or (and (> _returnvalue _bounced_fuse_duration) (Variables|Default|GetBounce%20Reduces%20Fuse)) (and (< _returnvalue _bounced_fuse_duration) (Variables|Default|GetBounce%20Increases%20Fuse)))
      (Utilities|Time|SetTimerbyEvent (delegate Custom|Trigger%20Explode) (Variables|Default|GetBounced%20Fuse%20Duration)))))

(event Custom|Trigger%20Explode
  (Class|URProjectile|Explode (Transformation|GetActorLocation) (Math|Vector|GetForwardVector (Transformation|GetActorRotation))))

(event EventBeginPlay
  ;[0 1 1] Manual explosion 6s after spawn
  (bind _returnvalue (Utilities|Time|SetTimerbyEvent (delegate Custom|Trigger%20Explode) (Variables|Default|GetInitial%20Fuse%20Duration)))
  (Variables|Default|SetTimerHandle _returnvalue))

(fn ConstructionScript)