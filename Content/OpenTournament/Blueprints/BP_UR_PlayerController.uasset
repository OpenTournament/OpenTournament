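; BP_UR_PlayerController is the player controller Blueprint for OpenTournament, handling basic input mode and opening in-game UI.
; On BeginPlay it runs the parent logic, then sets input to game-only.
; The ShowChatHistory and ShowIngameMenu input actions each create a fresh message history or in-game menu widget owned by the controller and call its Show function.
; A TODO notes chat history should also work in the main menu.
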(event EventBeginPlay
  (|CallParentFunction)
  (Input|SetInputModeGameOnly self))

(event Input|ActionEvents|InputActionShowChatHistory
  (params (Key :type Key%20Structure :default "None"))
  ;[1 1 1] InputAction Show Chat History
  ; TODO: this needs to work in main menu as well somehow
  (:Pressed
    (bind _returnvalue (UserInterface|CreateWidget "/Game/OpenTournament/UI/BP_Widget_MessageHistory.BP_Widget_MessageHistory_C" self))
    (Class|URWidgetBaseMenu|Show _returnvalue)))

(event Input|ActionEvents|InputActionShowIngameMenu
  (params (Key :type Key%20Structure :default "None"))
  ;[1 1 1] InputAction Show Ingame Menu
  (:Pressed
    (bind _returnvalue (UserInterface|CreateWidget "/Game/OpenTournament/UI/IngameMenu/BP_Widget_IngameMenu.BP_Widget_IngameMenu_C" self))
    (Class|URWidgetBaseMenu|Show _returnvalue)))

(fn ConstructionScript)