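; Base Blueprint for weapon pickups in OpenTournament, handling the pickup's mesh and its visual effects.
; The construction script sets the skeletal mesh from the configured weapon class and assigns it as the rotating component when that mesh is valid.
; Availability changes call the parent, then toggle mesh visibility including children.
; Pickup and respawn events each activate their own effect component.
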(event EventShowPickupAvailable
  (params (bAvailable :type Boolean))
  (|CallParentFunction bAvailable)
  (Rendering|SetVisibility (Variables|Default|GetPickupMesh) bAvailable true))

(event EventPlayPickupEffects
  (Components|Activation|Activate (Variables|Default|GetPickupEffect) true))

(event EventPlayRespawnEffects
  (Components|Activation|Activate (Variables|Default|GetRespawnEffect) true))

(fn ConstructionScript
  (Class|SkinnedMeshComponent|SetSkeletalMesh (Variables|Default|GetPickupMesh) (Class|URWeaponBase|GetMeshforWeapon (Variables|Default|GetWeaponClass)) true)
  (Utilities|IsValid (Variables|/Script/Engine.SkinnedMeshComponent|GetSkeletalMesh (Variables|Default|GetPickupMesh))
    (:Is%20Valid
      (Variables|Default|SetRotatingComponent (Variables|Default|GetPickupMesh)))
    (:Is%20Not%20Valid
      (Variables|Default|SetRotatingComponent 0))))