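; Base health pickup Blueprint that handles the visual feedback of a health item.
; Availability changes call the parent logic and toggle visibility of the pickup mesh and its children.
; Pickup and respawn events each activate their own effect component.
; The construction script assigns the pickup mesh as the rotating component.
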(event EventShowPickupAvailable
  (params (bAvailable :type Boolean))
  (|CallParentFunction bAvailable)
  (Rendering|SetVisibility (Variables|Default|GetPickupMesh) bAvailable true))

(event EventPlayPickupEffects
  (Components|Activation|Activate (Variables|Default|GetPickupEffect) true))

(event EventPlayRespawnEffects
  (Components|Activation|Activate (Variables|Default|GetRespawnEffect) true))

(fn ConstructionScript
  (Variables|Default|SetRotatingComponent (Variables|Default|GetPickupMesh)))