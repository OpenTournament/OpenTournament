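; Player character Blueprint for OpenTournament that adds voice sounds and a simple idle behavior on top of its parent class.
; Tick makes an uncontrolled character jump roughly every four seconds, using a time modulo check with a tolerance window.
; Jumping plays the CharacterVoice jump sound, while landing at high vertical speed plays a hardcoded male effort sound.
; The dodge handler is empty, and a crouch/uncrouch chain is left unconnected.
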(event Custom|OnDodge_1
  (params (DodgeLocation :type Vector%20%28by%20ref%29) (DodgeDir :type Vector%20%28by%20ref%29)))

(event Custom|OnJumped_1
  (Audio|PlaySoundatLocation (.JumpSound (Utilities|Struct|BreakCharacterVoice (Variables|Default|GetCharacterVoice))) (Transformation|GetActorLocation) "0, 0, 0" 1.0 1.0 0.0 0 0 0))

(event Custom|OnLanded_1
  (params (Hit :type Hit%20Result%20Structure%20%28by%20ref%29))
  (if (> (Math|Float|Absolute(Float) (.Z (Math|Vector|BreakVector (Transformation|GetVelocity)))) 1.2e+03)
    (Audio|PlaySoundatLocation "/Game/OpenTournament/Audio/Voices/General/A_Voice_Generic_Male_1_Landed_Effort.A_Voice_Generic_Male_1_Landed_Effort" (.Location (Collision|BreakHitResult Hit)) "0, 0, 0" 1.0 1.0 0.0 0 0 0)))

(event EventBeginPlay)

(event Collision|EventActorBeginOverlap
  (params (OtherActor :type Actor%20Object%20Reference)))

(event EventTick
  (params (DeltaSeconds :type Float%20%28single-precision%29))
  (if (and (not (Class|Pawn|IsControlled)) (Math|Float|NearlyEqual(Float) (Math|Float|%(Float) (Utilities|Time|GetTimeSeconds) 4.0) 0.0 0.1))
    (Character|Jump)))

(fn ConstructionScript)