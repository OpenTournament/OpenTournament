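; BP_AngleCalculator is a helper actor that displays the interior angles of a right triangle defined by its VerticalExtent and HorizontalExtent components.
; The construction script takes their absolute relative Z and Y offsets as side lengths and derives the hypotenuse via Pythagoras.
; The law of sines then gives each angle in degrees, written to two text components.
; The event graph holds only disabled placeholder events.
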(event EventBeginPlay)

(event Collision|EventActorBeginOverlap
  (params (OtherActor :type Actor%20Object%20Reference)))

(event EventTick
  (params (DeltaSeconds :type Float%20%28single-precision%29)))

(fn ConstructionScript
  (Variables|Default|SetLengthVertical (Math|Float|Absolute(Float) (.Z (Math|Vector|BreakVector (Variables|/Script/Engine.SceneComponent|GetRelativeLocation (Variables|Default|GetVerticalExtent))))))
  (Variables|Default|SetLengthHorizontal (Math|Float|Absolute(Float) (.Y (Math|Vector|BreakVector (Variables|/Script/Engine.SceneComponent|GetRelativeLocation (Variables|Default|GetHorizontalExtent))))))
  (CallFunction|SetLengthHypotenuse (Variables|Default|GetLengthVertical) (Variables|Default|GetLengthHorizontal))
  (Rendering|Components|TextRender|SetText (Variables|Default|GetText_AngleFromHorizontal) (Utilities|Text|ToText(Float) (CallFunction|CalculateTriangleInteriorAngle (Variables|Default|GetLengthVertical)) "HalfToEven"))
  (Rendering|Components|TextRender|SetText (Variables|Default|GetText_AngleFromVertical) (Utilities|Text|ToText(Float) (CallFunction|CalculateTriangleInteriorAngle (Variables|Default|GetLengthHorizontal)) "HalfToEven")))

(fn CalculateTriangleInteriorAngle
  (params (LengthOfSide :type Float%20%28single-precision%29))
  (return (Class|KismetMathLibrary|DegAsin (* (/ (Math|Trig|Sin(Degrees) 9e+01) (Variables|Default|GetLengthHypoteneuse)) LengthOfSide))))

(fn SetLengthHypotenuse
  (params (A :type Float%20%28single-precision%29) (A2 :type Float%20%28single-precision%29))
  (Variables|Default|SetLengthHypoteneuse (Math|Float|Sqrt (+ (Math|Float|Square A) (Math|Float|Square A2)))))