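; OpenTournament character Blueprint that adds crouch sliding, with Left Ctrl bound to crouch.
; Each tick, key change and crouched landing checks crouch state and speed, toggling slide overrides for friction, acceleration, braking and ledge walk-off against movement class defaults.
; While sliding, Tick applies a downhill force from the floor normal, scaled by gravity and slope.
; Crouched landings project saved horizontal velocity onto the floor plane after a brief delay, preserving momentum.
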(event Custom|ToggleCrouchSliding
  (params (Enabled :type Boolean))
  (bind (_groundfriction _maxacceleration _brakingdecelerationwalking) (Utilities|GetClassDefaults "/Script/OpenTournament.UR_CharacterMovementComponent"))
  (bind _urmovementcomponent (Variables|Default|GetURMovementComponent))
  (bind _output_get (Variables|Default|SetbSliding Enabled))
  (Variables|/Script/Engine.CharacterMovementComponent|SetGroundFriction _urmovementcomponent (Math|Float|SelectFloat (Variables|Default|GetSlideFriction) _groundfriction _output_get))
  (Variables|/Script/Engine.CharacterMovementComponent|SetMaxAcceleration _urmovementcomponent (Math|Float|SelectFloat (* _maxacceleration (Variables|Default|GetSlideControl)) _maxacceleration _output_get))
  (Variables|/Script/Engine.CharacterMovementComponent|SetBrakingDecelerationWalking _urmovementcomponent (Math|Float|SelectFloat 0.0 _brakingdecelerationwalking _output_get))
  (Variables|/Script/Engine.CharacterMovementComponent|SetbCanWalkOffLedgesWhenCrouching _urmovementcomponent (Variables|Default|GetbSliding)))

(event Custom|CheckCrouchSliding
  (bind _urmovementcomponent (Variables|Default|GetURMovementComponent))
  (if (AI|Components|NavMovement|IsCrouching _urmovementcomponent)
    (if (> (Math|Vector|VectorLength (Variables|/Script/Engine.MovementComponent|GetVelocity _urmovementcomponent)) (+ (Utilities|GetClassDefaults "/Script/OpenTournament.UR_CharacterMovementComponent") 1e+01))
      (if (not (Variables|Default|GetbSliding))
        (CallFunction|ToggleCrouchSliding true))
      (else
        (if (Variables|Default|GetbSliding) :!label _label
          (CallFunction|ToggleCrouchSliding false))))
    (else
      (goto _label))))

(event EventOnLanded
  (params (Hit :type Hit%20Result%20Structure%20%28by%20ref%29))
  (bind _urmovementcomponent (Variables|Default|GetURMovementComponent))
  (bind _urmovementcomponent_2 (Variables|Default|GetURMovementComponent))
  (bind _currentfloor (Variables|/Script/Engine.CharacterMovementComponent|GetCurrentFloor _urmovementcomponent_2))
  (if (Variables|/Script/Engine.CharacterMovementComponent|GetbWantsToCrouch _urmovementcomponent)
    (Variables|Default|SetLandingVel (Math|Vector|MakeVector (.x (Variables|/Script/Engine.MovementComponent|GetVelocity _urmovementcomponent)) (.y (Variables|/Script/Engine.MovementComponent|GetVelocity _urmovementcomponent)) 0.0))
    (Utilities|FlowControl|RetriggerableDelay 0.01)
    (Variables|/Script/Engine.MovementComponent|SetVelocity _urmovementcomponent_2 (- (Variables|Default|GetLandingVel) (* (.impactnormal (.hitresult _currentfloor)) (Math|Vector|DotProduct (Variables|Default|GetLandingVel) (.impactnormal (.hitresult _currentfloor))))))
    (CallFunction|CheckCrouchSliding)))

(event EventTick
  (params (DeltaSeconds :type Float%20%28single-precision%29))
  (bind _urmovementcomponent (Variables|Default|GetURMovementComponent))
  (bind _currentfloor (Variables|/Script/Engine.CharacterMovementComponent|GetCurrentFloor _urmovementcomponent))
  (bind (_x _y) (Math|Vector|BreakVector (.impactnormal (.hitresult _currentfloor))))
  (CallFunction|CheckCrouchSliding)
  (if (Variables|Default|GetbSliding)
    (Physics|AddForce (Variables|Default|GetURMovementComponent) (* (Math|Vector|CrossProduct (.impactnormal (.hitresult _currentfloor)) (Math|Vector|CrossProduct (Math|Vector|Normalize (Math|Vector|MakeVector _x _y 0.0)) (Math|Vector|MakeVector 0.0 0.0 1.0))) (* (* (Components|Movement|GetGravityZ _urmovementcomponent) -2.5e+02) (Math|Vector|VectorLengthXY (.impactnormal (.hitresult _currentfloor))))))))

(event Input|KeyboardEvents|LeftCtrl
  (params (Key :type Key%20Structure :default "None"))
  (:Pressed
    (Character|Crouch)
    (CallFunction|CheckCrouchSliding :!label _label))
  (:Released
    (Character|UnCrouch)
    (goto _label)))

(fn ConstructionScript
  (|CallParentFunction))