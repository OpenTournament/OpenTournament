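; Test actor that opens the key binding menu when play begins, switching player 0 to UI-only input with an unlocked mouse.
; Tab adds a separate ControlsMenu widget to the viewport, but the node chain that creates and assigns that older input bindings widget is disconnected.
; A PrintKeys debug function prints the keys mapped to Jump from the input settings, though nothing in the graph calls it.
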(event EventBeginPlay
  (bind _returnvalue (Game|GetPlayerController 0))
  (bind _returnvalue_2 (UserInterface|CreateWidget "/Game/OpenTournament/UI/BP_Widget_NewKeyBindingMenu.BP_Widget_NewKeyBindingMenu_C" _returnvalue))
  (Class|URWidgetKeyBindingMenu|OpenMenu _returnvalue_2)
  (Input|SetInputModeUIOnly _returnvalue 0 "DoNotLock"))

(event Collision|EventActorBeginOverlap
  (params (OtherActor :type Actor%20Object%20Reference)))

(event EventTick
  (params (DeltaSeconds :type Float%20%28single-precision%29)))

(event Input|KeyboardEvents|Tab
  (params (Key :type Key%20Structure))
  (:Pressed
    (UserInterface|Viewport|AddtoViewport (Variables|Default|GetControlsMenu) 0)))

(fn ConstructionScript)

(fn PrintKeys
  (for (_array_element _array_index) (Class|InputSettings|GetActionMappingbyName (Class|InputSettings|GetInputSettings) "Jump")
    (Development|PrintString (Utilities|String|Append (Utilities|String|BuildString(Integer) (Utilities|String|ToString(Name) (.ActionName (Utilities|Struct|BreakInputActionKeyMapping _array_element))) ": " _array_index ": ") (Utilities|String|ToString(Text) (Class|KismetInputLibrary|KeyGetDisplayName (.Key (Utilities|Struct|BreakInputActionKeyMapping _array_element))))))))