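; Functional test that checks an actor teleporter moves and rotates a character correctly.
; On start it spawns an AI controller and character at the player start, possesses it, and sends it to the first destination actor.
; Shortly after the move finishes, it passes only if the character is within its capsule radius of the second destination and matches its rotation within tolerance, otherwise failing with a specific message.
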(event EventPrepareTest)

(event EventStartTest
  (CallFunction|SpawnControllerCharacterandPossess)
  (AI|AIMoveTo (Variables|Default|GetController) "0, 0, 0" (Variables|Default|GetDestinationActor1) -1.0 "Default" "Default" true true
    (:OnRequestFailed
      (Class|FunctionalTest|FinishTest "Failed" "Move to Teleporter Failed"))
    (:OnMoveFinished
      (Utilities|FlowControl|Delay 0.1)
      (if (<= (Math|Vector|Distance(Vector) (Transformation|GetActorLocation (Variables|Default|GetCharacter)) (Transformation|GetActorLocation (Variables|Default|GetDestinationActor2))) (Components|Capsule|GetScaledCapsuleRadius (Variables|/Script/Engine.Character|GetCapsuleComponent (Variables|Default|GetCharacter))))
        (if (Math|Rotator|Equal(Rotator) (Transformation|GetActorRotation (Variables|Default|GetCharacter)) (Transformation|GetActorRotation (Variables|Default|GetDestinationActor2)) 0.5)
          (Class|FunctionalTest|FinishTest "Succeeded" "Teleportation Succeeded")
          (else
            (Class|FunctionalTest|FinishTest "Failed" "Character Reached Teleporter, But Failed to Rotate relative to DestinationLocation")))
        (else
          (Class|FunctionalTest|FinishTest "Failed" "Character Reached Teleporter, But Failed to Move to DestinationLocation"))))))

(event EventTick
  (params (DeltaSeconds :type Float%20%28single-precision%29)))

(fn ConstructionScript)

(fn SpawnControllerCharacterandPossess
  (bind _returnvalue (Game|SpawnActorfromClass (Variables|Default|GetControllerClass) (Transformation|GetActorTransform (Variables|Default|GetPlayerStart)) "Undefined" 0 0))
  (bind _asaicontroller (Utilities|Casting|CastToAIController _returnvalue))
  (bind _output_get (Variables|Default|SetController _asaicontroller))
  (bind _returnvalue_2 (Game|SpawnActorfromClass (Variables|Default|GetCharacterClass) (Transformation|GetActorTransform (Variables|Default|GetPlayerStart)) "Undefined" _output_get 0))
  (bind _ascharacter (Utilities|Casting|CastToCharacter _returnvalue_2))
  (Variables|Default|SetCharacter _ascharacter)
  (Pawn|Possess (Variables|Default|GetController) (Variables|Default|GetCharacter)))